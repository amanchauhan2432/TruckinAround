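; BP_Box is a pickup box that offers itself to a BP_Character entering its overlap volume.
; Begin overlap sets the character's CanPickup, shows a "Press P to pickup" prompt, and assigns itself as BoxRef after a tiny delay.
; End overlap clears CanPickup and the prompt on the cached character, leaving BoxRef set.
; HideBox creates a dynamic material and drives its Opacity parameter with a timeline.
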(event `self.Box.OnComponentBeginOverlap`
  (params (OverlappedComponent :type "PrimitiveComponent Object Reference") (OtherActor :type "Actor Object Reference") (OtherComp :type "PrimitiveComponent Object Reference") (OtherBodyIndex :type Integer) (bFromSweep :type Boolean) (SweepResult :type "HitResult Structure (by ref)"))
  (bind _asbp_character (cast `/Game/Blueprints/Character/BP_Character` OtherActor))
  (bind _output_get (set `self.Character Ref` _asbp_character))
  (set `/Game/Blueprints/Character/BP_Character.Can Pickup` true _output_get)
  (`KismetSystemLibrary.Delay` 1e-06)
  (set `/Game/Blueprints/Character/BP_Character.Box Ref` self (`self.Character Ref`))
  (`/Game/Blueprints/Character/BP_Character.Update Text` (`self.Character Ref`) "Press P to pickup" "Visible"))

(event `self.Box.OnComponentEndOverlap`
  (params (OverlappedComponent :type "PrimitiveComponent Object Reference") (OtherActor :type "Actor Object Reference") (OtherComp :type "PrimitiveComponent Object Reference") (OtherBodyIndex :type Integer))
  (bind _character_ref (`self.Character Ref`)
    (:`then`
      (set `/Game/Blueprints/Character/BP_Character.Can Pickup` false _character_ref)
      (`/Game/Blueprints/Character/BP_Character.Update Text` _character_ref "" "Collapsed"))
    (:`else`)))

(event `Hide Box`
  (bind _boxmesh (`self.BoxMesh`))
  ;[1 1 1] Hide the box
  (`PrimitiveComponent.CreateDynamicMaterialInstance` _boxmesh 0 "/Game/Assets/AssetsvilleTown/Materials/MasterMaterials/M_BoxBase.M_BoxBase" "None")
  (bind (_direction _alpha) (`Timeline|T_Opacity`)
    (:`Update`
      (`MeshComponent.SetScalarParameterValueOnMaterials` _boxmesh "Opacity" _alpha))))

(fn `UserConstructionScript`)