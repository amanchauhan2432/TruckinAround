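; Truck job marker actor that spawns a truck at its transform and handles that truck's pickup and parking.
; Pickup and parking switch off the Niagara marker, fade the location widget and have the character show the next random truck or location.
; Parking also teleports BP_Vehicle beside the truck, using a line trace that retries at a negative offset when blocked.
; It then pays a random wallet reward and destroys truck and marker after a delay.
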(event `self.ReceiveBeginPlay`
  (`|SpawnActorFromClass` (`self.Truck Class`) (`self.GetTransform`) "Undefined" "MultiplyWithRoot" null null))

(event `Event Truck Pickup`
  (params (`Truck Ref` :type "/Game/Blueprints/Vehicle/BP_Vehicle Object Reference"))
  ;[1 1 1] When the truck gets picked up
  (`ActorComponent.SetActive` (`self.NS_TruckDrop`) false false)
  (`self.Hide Widget`)
  (bind _character_ref (`self.Character Ref`)
    (:`then`
      (`/Game/Blueprints/Character/BP_Character.Show Random Truck` _character_ref false (`GameplayStatics.GetObjectClass` `Truck Ref`) "/Game/Assets/Textures/T_DropLocation.T_DropLocation" (struct :`R` 0.005605 :`G` 0.701102 :`A` 1.0))
      (`KismetSystemLibrary.Delay` 1.0)
      (`self.K2_DestroyActor`))
    (:`else`)))

(event `Event Truck Parked`
  (params (`Truck Ref` :type "/Game/Blueprints/Vehicle/BP_Vehicle Object Reference"))
  ;[1 1 1] When the truck gets parked
  (bind _character_ref (`self.Character Ref`)
    (:`then`
      (`/Game/Blueprints/Character/BP_Character.Show Random Location` _character_ref true "ECR_Ignore" "/Game/Assets/Textures/T_PickLocation.T_PickLocation" (struct :`R` 0.7 :`G` 0.030615 :`B` 0.156259 :`A` 1.0))
      (`ActorComponent.SetActive` (`self.NS_TruckDrop`) false false)
      (`self.Hide Widget`)
      (`self.Teleport Truck ` `Truck Ref`)
      (`self.Update Wallet`)
      (`KismetSystemLibrary.Delay` 10.0)
      (`self.K2_DestroyActor` `Truck Ref`)
      (`self.K2_DestroyActor`))
    (:`else`)))

(fn `Hide Widget`
  (bind _aswbp_location (cast `/Game/Widgets/WBP_Location` (`WidgetComponent.GetWidget` (`self.Widget`))))
  (`UserWidget.PlayAnimation` _aswbp_location (`/Game/Widgets/WBP_Location.FadeOut` _aswbp_location) 0.0 1 "Forward" 1.0 false))

(fn `Teleport Truck `
  (params (`Truck Ref` :type "Actor Object Reference"))
  (locals (Multiplier :type "Float (double-precision)" :default 900.0))
  (bind _returnvalue (`self.K2_GetActorLocation` `Truck Ref`))
  (bind _returnvalue_2 (+ _returnvalue (* (`self.GetActorRightVector` `Truck Ref`) (`local.Multiplier`))))
  (bind (_outhit _returnvalue_3) (`KismetSystemLibrary.LineTraceSingle` _returnvalue _returnvalue_2 "TraceTypeQuery1" :!label _label))
  (if _returnvalue_3
    (set `local.Multiplier` -900.0)
    (goto _label)
    (else
      (bind _returnvalue_4 (`GameplayStatics.GetActorOfClass` "/Game/Blueprints/Vehicle/BP_Vehicle.BP_Vehicle_C"))
      (`self.K2_TeleportTo` _returnvalue_4 _returnvalue_2 (`self.K2_GetActorRotation` `Truck Ref`)))))

(fn `Update Wallet`
  (bind _foundwidgets (`WidgetBlueprintLibrary.GetAllWidgetsOfClass` "/Game/Widgets/WBP_HUD.WBP_HUD_C"))
  (`/Game/Widgets/WBP_HUD.Update Wallet` (`|GetArrayItem` _foundwidgets) (`KismetMathLibrary.RandomFloatInRange` 5.5 8.0)))

(fn `Update Widget`
  (params (`Location Image` :type "Object Object Reference"))
  (bind _aswbp_location (cast `/Game/Widgets/WBP_Location` (`WidgetComponent.GetWidget` (`self.Widget`))))
  (`Image.SetBrush` (`/Game/Widgets/WBP_Location.Location_Img` _aswbp_location) (make `SlateBrush` "Image" "NoTile" "NoMirror" (struct :`X` 32.0 :`Y` 32.0) (struct) (struct :`SpecifiedColor` (struct :`R` 1.0 :`G` 1.0 :`B` 1.0 :`A` 1.0) :`ColorUseRule` "UseColor_Specified") (struct :`CornerRadii` (struct) :`Color` (struct :`SpecifiedColor` (struct) :`ColorUseRule` "UseColor_Specified") :`RoundingType` "HalfHeightRadius") (`local.Location Image`))))

(fn `UserConstructionScript`)