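; BP_Drop is a location marker for box deliveries that serves as a pickup point, spawning a BP_Box when SpawnBox is set, or as a drop point.
; A box leaving the pickup sphere fades the marker and has CharacterRef show a random drop location.
; A box entering the sphere snaps to center and, with a valid CharacterRef, notifies it, pays a random HUD wallet reward, then destroys box and marker.
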(event `self.ReceiveBeginPlay`
  (bind (_returnvalue_x _returnvalue_y) (`KismetMathLibrary.BreakVector` (`self.K2_GetActorLocation`)))
  (if (`self.Spawn Box`)
    (`|SpawnActorFromClass` "/Game/Blueprints/BP_Box.BP_Box_C" (`KismetMathLibrary.MakeTransform` (`KismetMathLibrary.MakeVector` _returnvalue_x _returnvalue_y 32.0)) "Undefined" "MultiplyWithRoot" null null)
    (`PrimitiveComponent.SetCollisionResponseToChannel` (`self.Sphere`) "ECC_Pawn" (`self.New Response`))))

(event `self.Sphere.OnComponentBeginOverlap`
  (params (OverlappedComponent :type "PrimitiveComponent Object Reference") (OtherActor :type "Actor Object Reference") (OtherComp :type "PrimitiveComponent Object Reference") (OtherBodyIndex :type Integer) (bFromSweep :type Boolean) (SweepResult :type "HitResult Structure (by ref)"))
  (bind (_returnvalue_x _returnvalue_y) (`KismetMathLibrary.BreakVector` (`self.K2_GetActorLocation`)))
  ;[1 1 1] When the box gets dropped
  (bind _asbp_box (cast `/Game/Blueprints/BP_Box` OtherActor))
  (`self.K2_SetActorLocation` _asbp_box (`KismetMathLibrary.MakeVector` _returnvalue_x _returnvalue_y 32.0) false false)
  (bind _character_ref (`self.Character Ref`)
    (:`then`
      (`/Game/Blueprints/Character/BP_Character.Box Or Truck` _character_ref)
      (`ActorComponent.SetActive` (`self.NS_DropPoint`) false false)
      (`/Game/Blueprints/BP_Box.Hide Box` _asbp_box)
      (`self.Hide Widget`)
      (`self.Update Wallet`)
      (`KismetSystemLibrary.Delay` 1.0)
      (`self.K2_DestroyActor` _asbp_box)
      (`self.K2_DestroyActor`))
    (:`else`)))

(event `self.Sphere.OnComponentEndOverlap`
  (params (OverlappedComponent :type "PrimitiveComponent Object Reference") (OtherActor :type "Actor Object Reference") (OtherComp :type "PrimitiveComponent Object Reference") (OtherBodyIndex :type Integer))
  ;[1 1 1] When the box gets picked up
  (cast `/Game/Blueprints/BP_Box` OtherActor)
  (if (`self.Spawn Box`)
    (`ActorComponent.SetActive` (`self.NS_DropPoint`) false false)
    (`self.Hide Widget`)
    (bind _character_ref (`self.Character Ref`)
      (:`then`
        (`/Game/Blueprints/Character/BP_Character.Show Random Location` _character_ref false "ECR_Block" "/Game/Assets/Textures/T_DropLocation.T_DropLocation" (struct :`R` 0.005498 :`G` 0.7 :`A` 1.0))
        (`KismetSystemLibrary.Delay` 1.0)
        (`self.K2_DestroyActor`))
      (:`else`))))

(fn `Hide Widget`
  (bind _aswbp_location (cast `/Game/Widgets/WBP_Location` (`WidgetComponent.GetWidget` (`self.Widget`))))
  (`UserWidget.PlayAnimation` _aswbp_location (`/Game/Widgets/WBP_Location.FadeOut` _aswbp_location) 0.0 1 "Forward" 1.0 false))

(fn `Update Wallet`
  (bind _foundwidgets (`WidgetBlueprintLibrary.GetAllWidgetsOfClass` "/Game/Widgets/WBP_HUD.WBP_HUD_C"))
  (`/Game/Widgets/WBP_HUD.Update Wallet` (`|GetArrayItem` _foundwidgets) (`KismetMathLibrary.RandomFloatInRange` 1.0 4.0)))

(fn `Update Widget`
  (params (`Location Image` :type "Object Object Reference"))
  (bind _aswbp_location (cast `/Game/Widgets/WBP_Location` (`WidgetComponent.GetWidget` (`self.Widget`))))
  (`Image.SetBrush` (`/Game/Widgets/WBP_Location.Location_Img` _aswbp_location) (make `SlateBrush` "Image" "NoTile" "NoMirror" (struct :`X` 32.0 :`Y` 32.0) (struct) (struct :`SpecifiedColor` (struct :`R` 1.0 :`G` 1.0 :`B` 1.0 :`A` 1.0) :`ColorUseRule` "UseColor_Specified") (struct :`CornerRadii` (struct) :`Color` (struct :`SpecifiedColor` (struct) :`ColorUseRule` "UseColor_Specified") :`RoundingType` "HalfHeightRadius") (`local.Location Image`))))

(fn `UserConstructionScript`)